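; BP_EntityBase is an entity base with RPG-style stats, damage and level-up growth, keyed by an Archetype row name.
; BeginPlay finds the DT_Base_Stats row and sets the stats, though to literal zeros, with DEF set twice and DEX never.
; LevelUp finds the DT_Growth_Rates row and rolls randomly to increment each stat, with every threshold at zero.
; AnyDamage subtracts damage from CHP, which BeginPlay leaves unset.
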(event Custom|LevelUp
  (bind _archetype (Variables|BaseStats|GetArchetype))
  (Class|DataTableFunctionLibrary|DoesDataTableRowExist "/Game/MilesFortunae/Blueprints/DT_Growth_Rates.DT_Growth_Rates" _archetype)
  (if true
    (Utilities|GetDataTableRow "/Game/MilesFortunae/Blueprints/DT_Growth_Rates.DT_Growth_Rates" _archetype
      (:then
        (Utilities|FlowControl|Sequence
          (:then_0
            (if (<= (Math|Random|RandomFloat) 0.0)
              (Math|Float|IncrementFloat (Variables|BaseStats|GetmHP))))
          (:then_1
            (if (<= (Math|Random|RandomFloat) 0.0)
              (Math|Float|IncrementFloat (Variables|BaseStats|GetSTR))))
          (:then_2
            (if (<= (Math|Random|RandomFloat) 0.0)
              (Math|Float|IncrementFloat (Variables|BaseStats|GetDEX))))
          (:then_3
            (if (<= (Math|Random|RandomFloat) 0.0)
              (Math|Float|IncrementFloat (Variables|BaseStats|GetSPD))))
          (:then_4
            (if (<= (Math|Random|RandomFloat) 0.0)
              (Math|Float|IncrementFloat (Variables|BaseStats|GetINT))))
          (:then_5
            (if (<= (Math|Random|RandomFloat) 0.0)
              (Math|Float|IncrementFloat (Variables|BaseStats|GetDEF))))
          (:then_6
            (if (<= (Math|Random|RandomFloat) 0.0)
              (Math|Float|IncrementFloat (Variables|BaseStats|GetRES)))))))))

(event EventBeginPlay
  (bind _archetype (Variables|BaseStats|GetArchetype))
  (Class|DataTableFunctionLibrary|DoesDataTableRowExist "/Game/MilesFortunae/Blueprints/DT_Base_Stats.DT_Base_Stats" _archetype)
  (if true
    (Utilities|GetDataTableRow "/Game/MilesFortunae/Blueprints/DT_Base_Stats.DT_Base_Stats" _archetype
      (:then
        (Variables|BaseStats|SetmHP 0.0)
        (Variables|BaseStats|SetSTR 0.0)
        (Variables|BaseStats|SetDEF 0.0)
        (Variables|BaseStats|SetSPD 0.0)
        (Variables|BaseStats|SetINT 0.0)
        (Variables|BaseStats|SetDEF 0.0)
        (Variables|BaseStats|SetRES 0.0)))))

(event Game|Damage|EventAnyDamage
  (params (Damage :type Float%20%28single-precision%29) (DamageType :type Damage%20Type%20Object%20Reference) (InstigatedBy :type Controller%20Object%20Reference) (DamageCauser :type Actor%20Object%20Reference))
  (Variables|BaseStats|SetcHP (- (Variables|BaseStats|GetcHP) Damage)))

(fn ConstructionScript)