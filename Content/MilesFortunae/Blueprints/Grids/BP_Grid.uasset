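; BP_Grid is an actor that builds a tile grid centred on its location at construction time, using one instanced static mesh component.
; SpawnGrid clears old instances, applies the flat mesh and material from DT_GridShapes for the chosen shape, then adds instances row by column.
; The centre snaps to tile scale, and the corner offset accounts for even or odd lengths.
; Tile scaling always reads one fixed shape's mesh size.
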(event EventBeginPlay)

(event Collision|EventActorBeginOverlap
  (params (OtherActor :type Actor%20Object%20Reference)))

(event EventTick
  (params (DeltaSeconds :type Float%20%28single-precision%29)))

(fn ConstructionScript
  (CallFunction|SpawnGrid (Transformation|GetActorLocation) (Variables|Default|GetTile%20Scaler) (Variables|Default|GetGrid%20length) (Variables|Default|GetGrid%20Shape)))

(fn SpawnGrid
  (params (Centre :type Vector) (Scaler :type Vector) (Size :type Vector%202D%20Structure) (Shape :type E_shapeDataIndex%20Enum :default "NewEnumerator0"))
  (bind _instancedstaticmesh (Variables|Default|GetInstancedStaticMesh))
  (Variables|Default|SetGrid%20Centre Centre)
  (Variables|Default|SetTile%20Scaler Scaler)
  (Variables|Default|SetGrid%20length (Class|KismetMathLibrary|ToRounded2D Size))
  (bind _output_get (Variables|Default|SetGrid%20Shape Shape))
  (CallFunction|DestroyInstances)
  (Components|StaticMesh|SetStaticMesh _instancedstaticmesh (.FlatMesh (Utilities|Struct|BreakS_GridShape_Data (CallFunction|GetCurrentShapeData _output_get))))
  (Rendering|Material|SetMaterial _instancedstaticmesh 0 (.FlatMaterial (Utilities|Struct|BreakS_GridShape_Data (CallFunction|GetCurrentShapeData _output_get))))
  (bind (_bl _centre) (CallFunction|CalcGridCentreandLeft))
  (Variables|Default|SetGrid%20Centre _centre)
  (Variables|Default|SetgridBottomLCorner _bl)
  (for _index (range 0 (- (Math|Float|Round (.x (Variables|Default|GetGrid%20length))) 1))
    (LocalVariables|Setx _index)
    (for _index_2 (range 0 (- (Math|Float|Round (.y (Variables|Default|GetGrid%20length))) 1))
      (LocalVariables|Sety _index_2)
      (bind _output_get_2 (LocalVariables|SettileTransform (Math|Transform|MakeTransform (+ (+ (Variables|Default|GetgridBottomLCorner) (* (Math|Vector|MakeVector (LocalVariables|Getx) (LocalVariables|Gety) 0.0) (Variables|Default|GetTile%20Scaler))) "0.000000,0.000000,2.000000") "0, 0, 0" (/ (Variables|Default|GetTile%20Scaler) (.MeshSize (Utilities|Struct|BreakS_GridShape_Data (CallFunction|GetCurrentShapeData "NewEnumerator1")))))))
      (Components|InstancedStaticMesh|AddInstance (Variables|Default|GetInstancedStaticMesh) _output_get_2 true))))

(fn GetCurrentShapeData
  (params (Enumerator :type E_shapeDataIndex%20Enum :default "NewEnumerator0"))
  (bind _returnvalue (Utilities|GetDataTableRow "/Game/MilesFortunae/Blueprints/Grids/DT_GridShapes.DT_GridShapes" (Utilities|String|StringToName (Utilities|String|EnumtoString Enumerator)))
    (:then
      _)
    (:RowNotFound
      _))
  (return _returnvalue))

(fn DestroyInstances
  (Components|InstancedStaticMesh|ClearInstances (Variables|Default|GetInstancedStaticMesh))
  (return 0))

(fn CalcGridCentreandLeft
  (bind _grid_length (Variables|Default|GetGrid%20length))
  (LocalVariables|SetvectorC (CallFunction|SnapVectortoVector (Variables|Default|GetGrid%20Centre) (Variables|Default|GetTile%20Scaler)))
  (return (- (LocalVariables|GetvectorC) (* (Variables|Default|GetTile%20Scaler) (/ (- (Variables|Default|GetGrid%20length) (Math|Vector2D|MakeVector2D (Math|Float|SelectFloat 0.0 1.0 (CallFunction|IsFloatEven (.x _grid_length))) (Math|Float|SelectFloat 0.0 1.0 (CallFunction|IsFloatEven (.y _grid_length))))) "(X=2.000000,Y=2.000000)"))) (LocalVariables|GetvectorC)))