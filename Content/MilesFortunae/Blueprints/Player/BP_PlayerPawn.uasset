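; BP_PlayerPawn is a free-moving camera pawn with a spring arm that the player pans, rotates and zooms.
; Axis inputs shift a location goal along the actor's right and forward vectors and adjust a clamped zoom goal, while rotate presses step a yaw goal.
; Tick interpolates actor location, rotation and spring arm length toward those goals for smoothed motion, without sweeping for collision.
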(event EventTick
  (params (DeltaSeconds :type Float%20%28single-precision%29))
  (bind _springarm (Variables|Default|GetSpringArm))
  (Variables|/Script/Engine.SpringArmComponent|SetTargetArmLength _springarm (Math|Interpolation|FInterpTo (Variables|/Script/Engine.SpringArmComponent|GetTargetArmLength _springarm) (Variables|movements|GetzoomGoal) DeltaSeconds (Variables|Spinvalues|GetzoomInterpSpeed)))
  (Transformation|SetActorLocation (Math|Interpolation|VInterpTo (Transformation|GetActorLocation) (Variables|movements|GetlocationGoal) DeltaSeconds (Variables|Spinvalues|GetmoveInterpSpeed)) false false)
  (Transformation|SetActorRotation (Math|Interpolation|RInterpTo (Transformation|GetActorRotation) (Variables|Movements|Getrotation_Goal) DeltaSeconds (Variables|Spinvalues|GetrotateInterpSpeed))))

(event EventBeginPlay
  ;[0 0 0] Init
  (Variables|movements|SetlocationGoal (Transformation|GetActorLocation))
  (Variables|movements|SetzoomGoal (Variables|/Script/Engine.SpringArmComponent|GetTargetArmLength (Variables|Default|GetSpringArm)))
  (Variables|Movements|Setrotation_Goal (Transformation|GetActorRotation)))

(event Input|ActionEvents|InputActionInputAction_RotateL
  (params (Key :type Key%20Structure :default "None"))
  ;[0 0 0] Rotate Cam
  (:Pressed
    (Variables|Movements|Setrotation_Goal (Math|Rotator|CombineRotators (Variables|Movements|Getrotation_Goal) (Math|Rotator|MakeRotator 0.0 0.0 (Variables|spinvalues|GetrotateSpeed))))))

(event Input|ActionEvents|InputActionInputAction_RotateR
  (params (Key :type Key%20Structure :default "None"))
  ;[0 0 0] Rotate Cam
  (:Pressed
    (Variables|Movements|Setrotation_Goal (Math|Rotator|CombineRotators (Variables|Movements|Getrotation_Goal) (Math|Rotator|MakeRotator 0.0 0.0 (* (Variables|spinvalues|GetrotateSpeed) -1.0))))))

(event Input|AxisEvents|InputAxisInputAxis_Zoom
  (params (AxisValue :type Float%20%28single-precision%29))
  ;[0 0 0] Zoom
  (Variables|movements|SetzoomGoal (Math|Float|Clamp(Float) (+ (* AxisValue (Variables|Spinvalues|GetzoomSpeed)) (Variables|movements|GetzoomGoal)) (Variables|Spinvalues|GetzoomMin) (Variables|Spinvalues|GetzoomMax))))

(event Input|AxisEvents|InputAxisInputAxis_LR
  (params (AxisValue :type Float%20%28single-precision%29))
  ;[0 0 0] Move camera left/right
  (Variables|movements|SetlocationGoal (+ (Variables|movements|GetlocationGoal) (* (* AxisValue (Variables|spinvalues|GetmoveSpeed)) (Transformation|GetActorRightVector)))))

(event Input|AxisEvents|InputAxisInputAxis_Forward
  (params (AxisValue :type Float%20%28single-precision%29))
  ;[0 0 0] Move camera back/forth
  (Variables|movements|SetlocationGoal (+ (Variables|movements|GetlocationGoal) (* (* AxisValue (Variables|spinvalues|GetmoveSpeed)) (Transformation|GetActorForwardVector)))))

(fn ConstructionScript)