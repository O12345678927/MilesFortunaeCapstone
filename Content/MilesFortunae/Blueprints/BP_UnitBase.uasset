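; Base unit Blueprint that holds a combat unit's RPG stats, health, weapon and level.
; BeginPlay loads DT_BaseStats by Archetype and equips a default spear; weaponChange derives effective might, speed and hit from DT_Equipment, using INT or STR for might.
; AnyDamage subtracts raw damage from current HP.
; LevelUp rolls each stat against DT_StatGrowths chances and prints gains, without recomputing weapon-derived values or current HP.
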(event Custom|LevelUp
  ;[0 0 0] LevelUp
  (Math|Float|IncrementFloat (Variables|Stat|GetLvl)
    (:%20%20
      (bind _returnvalue (Utilities|GetDataTableRow "/Game/MilesFortunae/DataTables/DT_StatGrowths.DT_StatGrowths" (Variables|Stat|GetArchetype))
        (:then
          (Utilities|FlowControl|Sequence
            (:then_0
              (if (<= (Math|Random|RandomFloat) (.mhp _returnvalue))
                (Math|Float|IncrementFloat (Variables|Stat|GetmHP)
                  (:%20%20
                    (Development|PrintString "HP")))))
            (:then_1
              (if (<= (Math|Random|RandomFloat) (.str _returnvalue))
                (Math|Float|IncrementFloat (Variables|Stat|GetSTR)
                  (:%20%20
                    (Development|PrintString "STR")))))
            (:then_2
              (if (<= (Math|Random|RandomFloat) (.dex _returnvalue))
                (Math|Float|IncrementFloat (Variables|Stat|GetDEX)
                  (:%20%20
                    (Development|PrintString "DEX")))))
            (:then_3
              (if (<= (Math|Random|RandomFloat) (.spd _returnvalue))
                (Math|Float|IncrementFloat (Variables|Stat|GetSPD)
                  (:%20%20
                    (Development|PrintString "SPD")))))
            (:then_4
              (if (<= (Math|Random|RandomFloat) (.int _returnvalue))
                (Math|Float|IncrementFloat (Variables|Stat|GetINT)
                  (:%20%20
                    (Development|PrintString "INT")))))
            (:then_5
              (if (<= (Math|Random|RandomFloat) (.def _returnvalue))
                (Math|Float|IncrementFloat (Variables|Stat|GetDEF)
                  (:%20%20
                    (Development|PrintString "DEF")))))
            (:then_6
              (if (<= (Math|Random|RandomFloat) (.res _returnvalue))
                (Math|Float|IncrementFloat (Variables|Stat|GetRES)
                  (:%20%20
                    (Development|PrintString "RES")))))))))))

(event Custom|weaponChange
  ;[0 0 0] Change Weapon
  (if (== (Variables|Equipment|GetWeapon) (Variables|Equipment|GetintWeapon))
    (bind _returnvalue (Utilities|GetDataTableRow "/Game/MilesFortunae/DataTables/DT_Equipment.DT_Equipment" (Variables|Equipment|GetWeapon))
      (:then
        (Variables|Default|SeteMT (+ (.mt _returnvalue) (Variables|Stat|GetINT)))
        (Variables|Default|SeteSPD (- (Variables|Stat|GetSPD) (.wgt _returnvalue)))
        (Variables|Default|SeteHIT (+ (.hit _returnvalue) (* (Variables|Stat|GetDEX) 2.0)))))
    (else
      (bind _returnvalue_2 (Utilities|GetDataTableRow "/Game/MilesFortunae/DataTables/DT_Equipment.DT_Equipment" (Variables|Equipment|GetWeapon))
        (:then
          (Variables|Default|SeteMT (+ (.mt _returnvalue_2) (Variables|Stat|GetSTR)))
          (Variables|Default|SeteSPD (- (Variables|Stat|GetSPD) (.wgt _returnvalue_2)))
          (Variables|Default|SeteHIT (+ (.hit _returnvalue_2) (* (Variables|Stat|GetDEX) 2.0))))))))

(event EventBeginPlay
  ;[0 0 0] Init
  (bind _returnvalue (Utilities|GetDataTableRow "/Game/MilesFortunae/DataTables/DT_BaseStats.DT_BaseStats" (Variables|Stat|GetArchetype))
    (:then
      (Variables|Stat|SetmHP (.mhp _returnvalue))
      (Variables|Stat|SetcHP (.mhp _returnvalue))
      (Variables|Stat|SetSTR (.str _returnvalue))
      (Variables|Stat|SetDEX (.dex _returnvalue))
      (Variables|Stat|SetSPD (.spd _returnvalue))
      (Variables|Stat|SetINT (.int _returnvalue))
      (Variables|Stat|SetDEF (.def _returnvalue))
      (Variables|Stat|SetRES (.res _returnvalue))
      (Variables|Equipment|SetWeapon "spearOne")
      (CallFunction|WeaponChange))))

(event Game|Damage|EventAnyDamage
  (params (Damage :type Float%20%28single-precision%29) (DamageType :type Damage%20Type%20Object%20Reference) (InstigatedBy :type Controller%20Object%20Reference) (DamageCauser :type Actor%20Object%20Reference))
  ;[0 0 0] TakeDamage
  (Variables|Stat|SetcHP (- (Variables|Stat|GetcHP) Damage)))

(fn ConstructionScript)