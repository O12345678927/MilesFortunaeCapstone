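; BP_CombatManager resolves turn-based exchanges between an attacker and a defender using their stats.
; Combat flags whichever side's speed leads by at least TwoHit, then runs attack, counter and that side's follow-up; otherwise no attacks run, and flags are never reset.
; Attack hits when a 1–100 roll is at least EHIT minus DEX, subtracting EMT minus DEF from CHP, with debug prints for both outcomes.
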(event Custom|Combat
  (params (Attacker :type BP%20Unit%20Base%20Object%20Reference) (Defender :type BP%20Unit%20Base%20Object%20Reference))
  (bind _espd (Variables|/Game/MilesFortunae/Blueprints/BP_UnitBase.BP_UnitBase_C|GeteSPD Attacker))
  (bind _espd_2 (Variables|/Game/MilesFortunae/Blueprints/BP_UnitBase.BP_UnitBase_C|GeteSPD Defender))
  (bind _twohit (Variables|Default|GettwoHit))
  (if (>= _espd (+ _espd_2 _twohit))
    (Variables|Default|SetaDouble true)
    (CallFunction|Attack Attacker Defender :!label _label)
    (CallFunction|Attack Defender Attacker)
    (if (Variables|Default|GetaDouble)
      (CallFunction|Attack Attacker Defender)
      (elif (Variables|Default|GetdDouble)
        (CallFunction|Attack Defender Attacker)))
    (elif (>= _espd_2 (+ _espd _twohit))
      (Variables|Default|SetdDouble true)
      (goto _label))))

(event Custom|Attack
  (params (Attacker :type BP%20Unit%20Base%20Object%20Reference) (Defender :type BP%20Unit%20Base%20Object%20Reference))
  (if (>= (Math|Random|RandomIntegerinRange 1 100) (- (Variables|/Game/MilesFortunae/Blueprints/BP_UnitBase.BP_UnitBase_C|GeteHIT Attacker) (Variables|/Game/MilesFortunae/Blueprints/BP_UnitBase.BP_UnitBase_C|GetDEX Defender)))
    (bind _output_get (Variables|/Game/MilesFortunae/Blueprints/BP_UnitBase.BP_UnitBase_C|SetcHP Defender (- (Variables|/Game/MilesFortunae/Blueprints/BP_UnitBase.BP_UnitBase_C|GetcHP Defender) (- (Variables|/Game/MilesFortunae/Blueprints/BP_UnitBase.BP_UnitBase_C|GeteMT Attacker) (Variables|/Game/MilesFortunae/Blueprints/BP_UnitBase.BP_UnitBase_C|GetDEF Defender)))))
    (Development|PrintString (Utilities|String|ToString(Float) _output_get))
    (else
      (Development|PrintString "Hello"))))

(fn ConstructionScript)